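; Guard enemy Character that locks onto the first player seen by PawnSensing and chases them.
; Tick turns it toward the player and moves it; within AttachDis it moves forward or back at half input, flipped by a randomly re-armed timer.
; Any capsule overlap ragdolls it.
; Unconnected logic holds AI move-and-shoot and the timer for a routine that randomly hides player hand and gun parts or disables player movement.
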(event OnSeePawn(PawnSensing)
  (params (Pawn :type Pawn%20Object%20Reference))
  (Variables|Default|GetAs%20Player
    (:then)
    (:else
      (bind _asplayer (Utilities|Casting|CastToPlayer Pawn))
      (Variables|Default|SetAs%20Player _asplayer))))

(event OnComponentBeginOverlap(CapsuleComponent)
  (params (OverlappedComponent :type Primitive%20Component%20Object%20Reference) (OtherActor :type Actor%20Object%20Reference) (OtherComp :type Primitive%20Component%20Object%20Reference) (OtherBodyIndex :type Integer) (bFromSweep :type Boolean) (SweepResult :type Hit%20Result%20Structure%20%28by%20ref%29))
  (CallFunction|Ragdoll))

(event Custom|destroy_player
  (Utilities|FlowControl|Delay (Math|Random|RandomFloatinRange 1.0 1e+01))
  (CallFunction|FindPlayerComponents)
  (Utilities|FlowControl|Delay 2.0)
  (Utilities|FlowControl|Delay (Math|Random|RandomFloatinRange 1.0 1e+01))
  (CallFunction|FindPlayerComponents)
  (Utilities|FlowControl|Delay 2.0)
  (Utilities|FlowControl|Delay (Math|Random|RandomFloatinRange 1.0 1e+01))
  (CallFunction|FindPlayerComponents)
  (Utilities|FlowControl|Delay 2.0)
  (Utilities|FlowControl|Delay (Math|Random|RandomFloatinRange 1.0 1e+01))
  (CallFunction|FindPlayerComponents))

(event Custom|changestrafdirection
  (bind _isa (Utilities|FlowControl|FlipFlop)
    (:A
      _)
    (:B
      _))
  (Variables|Default|Setstrafright _isa)
  (Utilities|Time|SetTimerbyEvent (delegate Custom|changestrafdirection) (Math|Random|RandomFloatinRange 2.0 6.0)))

(event EventTick
  (params (DeltaSeconds :type Float%20%28single-precision%29))
  (bind _returnvalue (Transformation|GetActorLocation))
  (bind _as_player (Variables|Default|GetAs%20Player)
    (:then
      (if (> (Transformation|GetDistanceTo _as_player) (Variables|Default|Getattach_dis))
        (Pawn|Input|AddMovementInput (Math|Rotator|GetRotationXVector (Math|Rotator|MakeRotator 0.0 0.0 (.yaw (Math|Rotator|FindLookatRotation _returnvalue (+ (Transformation|GetActorLocation _as_player) "0, 0,100.000000"))))) 1.0 false)
        (Transformation|SetActorRotation (Math|Rotator|Lerp(Rotator) (Transformation|GetActorRotation) (Math|Rotator|MakeRotator 0.0 0.0 (.yaw (Math|Rotator|FindLookatRotation _returnvalue (+ (Transformation|GetActorLocation _as_player) "0, 0,100.000000")))) 0.5 true))
        (else
          (Pawn|Input|AddMovementInput (Math|Rotator|GetRotationXVector (Math|Rotator|FindLookatRotation _returnvalue (Transformation|GetActorLocation _as_player))) (Math|Float|SelectFloat 0.5 -0.5 (Variables|Default|Getstrafright)) false)
          (Transformation|SetActorRotation (Math|Rotator|Lerp(Rotator) (Transformation|GetActorRotation) (Math|Rotator|FindLookatRotation _returnvalue (Transformation|GetActorLocation _as_player)) 0.5 true)))))
    (:else)))

(event EventBeginPlay
  (CallFunction|Changestrafdirection))

(fn ConstructionScript)

(fn Ragdoll
  (Physics|SetSimulatePhysics (Variables|Character|GetMesh) true)
  (Pawn|Components|CharacterMovement|DisableMovement (Variables|Character|GetCharacterMovement))
  (Collision|SetCollisionEnabled (Variables|Collision|GetCapsuleComponent) "NoCollision")
  (Variables|Default|Setdisable true))

(fn FindPlayerComponents
  (bind _returnvalue (Game|GetPlayerCharacter 0))
  (bind _player_component (Variables|Default|Getplayer_component))
  (bind _player_component_2 (Variables|Default|Getplayer_component))
  (bind _outitem (Utilities|Array|Random _player_component))
  (bind _asplayer (Utilities|Casting|CastToPlayer _returnvalue))
  (bind _gun (Variables|/Game/Blueprint/Player.Player_C|Getgun _asplayer))
  (if (== _outitem 1)
    (Rendering|SetVisibility (Variables|/Game/Blueprint/Player.Player_C|Gethand_ _asplayer) false false)
    (Utilities|Array|RemoveIndex _player_component_2)
    (elif (== _outitem 2)
      (Rendering|SetVisibility (Variables|/Script/Engine.Actor|GetRootComponent (Variables|/Game/Blueprint/Player.Player_C|Getgun _asplayer)) false false)
      (Utilities|Array|RemoveIndex _player_component_2 1)
      (elif (== _outitem 3)
        (Pawn|Components|CharacterMovement|DisableMovement (Variables|/Script/Engine.Character|GetCharacterMovement _asplayer))
        (Utilities|Array|RemoveIndex _player_component_2 2)
        (elif (== _outitem 4)
          (Rendering|SetVisibility (Variables|/Game/models/gun_assets/gun/gun01_Blueprint.gun01_Blueprint_C|Getmagazine _gun) false false)
          (Utilities|Array|RemoveIndex _player_component_2 3)
          (elif (== _outitem 5)
            (Rendering|SetVisibility (Variables|/Script/Engine.Actor|GetRootComponent (Variables|/Game/models/gun_assets/gun/gun01_Blueprint.gun01_Blueprint_C|Getscope _gun)) false false)
            (Utilities|Array|RemoveIndex _player_component_2 4)
            (elif (== _outitem 6)
              (Rendering|SetVisibility (Variables|/Game/models/gun_assets/gun/gun01_Blueprint.gun01_Blueprint_C|GetammoText _gun) false false)
              (Utilities|Array|RemoveIndex _player_component_2 5))))))))