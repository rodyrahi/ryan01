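; Actor component that tracks and toggles attachment of a gun for a player character.
; A setup event stores references to the character, gun, hands and attachment.
; Attach and unattach events call the gun's own attach and unattach functions and maintain an attached flag, which guards against attaching twice.
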(event Custom|unattach
  ;[1 0 0.2409 1 75] Attachment
  (Default|Unattach (Variables|Default|Getgun))
  (Variables|Default|Setattachment_attached false))

(event Custom|get_player
  (params (character :type Character%20Object%20Reference) (gun :type Gun%20Blueprint%20Object%20Reference) (hands :type %20Object%20Reference) (attachment :type Attachment%20Blueprint%20Object%20Reference))
  (Variables|Default|Setcharacter character)
  (Variables|Default|Sethands hands)
  (Variables|Default|Setgun gun)
  (Variables|Default|Setattachment attachment))

(event Custom|attach
  ;[1 0 0.2409 1 75] Attachment
  (if (not (Variables|Default|Getattachment_attached))
    (Default|AttachGun (Variables|Default|Getgun))
    (Variables|Default|Setattachment_attached true)))